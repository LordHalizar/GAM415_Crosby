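; Base enemy for a retro FPS, drawn as a directional Paper2D flipbook sprite.
; Tick derives idle, moving, melee or ranged state from velocity and attack flags, then picks flipbook and sprite rotation from the player's relative angle using dot products.
; PawnSensing sets a timed CanSeePlayer flag and Blackboard key, turning the enemy toward the player.
; Delayed attack events line-trace melee damage or spawn projectiles; death increments the player's kill count.
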(event `self.ReceiveBeginPlay`
  (bind _asbp_first_person_character (cast `/Game/FirstPerson/Blueprints/BP_FirstPersonCharacter` (`GameplayStatics.GetPlayerCharacter` 0)))
  (set `self.PlayerReference` _asbp_first_person_character))

(event `self.ReceiveTick`
  (params (DeltaSeconds :type "Float (single-precision)"))
  (bind _returnvalue (`GameplayStatics.GetPlayerCharacter` 0))
  (bind _returnvalue_2 (`KismetMathLibrary.Normal` (- (`self.K2_GetActorLocation` _returnvalue) (`self.K2_GetActorLocation`))))
  (if (> (`KismetMathLibrary.VSize` (`MovementComponent.Velocity` (`self.CharacterMovement`))) 0.0)
    (if (`self.IsAttacking`)
      (switch `/Game/RetroFpsAssets/Enemies/AttackingState` (`self.AttackState`)
        (:`NewEnumerator0`
          (set `self.EnemyState` "NewEnumerator2"))
        (:`NewEnumerator1`
          (set `self.EnemyState` "NewEnumerator3")))
      (else
        (set `self.EnemyState` "NewEnumerator1")))
    (elif (`self.IsAttacking`)
      (switch `/Game/RetroFpsAssets/Enemies/AttackingState` (`self.AttackState`)
        (:`NewEnumerator0`
          (set `self.EnemyState` "NewEnumerator2"))
        (:`NewEnumerator1`
          (set `self.EnemyState` "NewEnumerator3")))
      (else
        (set `self.EnemyState` "NewEnumerator0"))))
  (if (`self.CanSeePlayer`)
    (`self.RotateTowardsPlayer`)
    (else
      (`/Engine/EditorBlueprintResources/StandardMacros.IsValid` _returnvalue
        (:`Is Valid`
          _))))
  (set `self.Degrees` (`KismetMathLibrary.DegAcos` (`KismetMathLibrary.Dot_VectorVector` (`self.GetActorForwardVector`) _returnvalue_2)))
  (if (< (`KismetMathLibrary.Dot_VectorVector` (`self.GetActorRightVector`) _returnvalue_2) 0.0)
    (`/Engine/EditorBlueprintResources/StandardMacros.CompareFloat` (`self.Degrees`) 180.0
      (:`>`
        (`SceneComponent.K2_SetRelativeRotation` (`self.PaperFlipbook`) (struct :`Yaw` -90.0) false false :!label _label)
        (`PaperFlipbookComponent.SetFlipbook` (`self.PaperFlipbook`) (`|GetArrayItem` (select `/Game/RetroFpsAssets/Enemies/EnemyState` (`self.EnemyState`) :`NewEnumerator0` (`self.FlipbooksIdles`) :`NewEnumerator1` (`self.FlipbooksMoving`) :`NewEnumerator2` (`self.FlipbooksMeleeAttacks`) :`NewEnumerator3` (`self.FlipbooksRangedAttacks`)))))
      (:`==`
        (goto _label))
      (:`<`
        (`/Engine/EditorBlueprintResources/StandardMacros.CompareFloat` (`self.Degrees`) 135.0
          (:`>`
            (`SceneComponent.K2_SetRelativeRotation` (`self.PaperFlipbook`) (struct :`Yaw` 135.0) false false :!label _label_2)
            (`PaperFlipbookComponent.SetFlipbook` (`self.PaperFlipbook`) (`|GetArrayItem` (select `/Game/RetroFpsAssets/Enemies/EnemyState` (`self.EnemyState`) :`NewEnumerator0` (`self.FlipbooksIdles`) :`NewEnumerator1` (`self.FlipbooksMoving`) :`NewEnumerator2` (`self.FlipbooksMeleeAttacks`) :`NewEnumerator3` (`self.FlipbooksRangedAttacks`)) 3)))
          (:`==`
            (goto _label_2))
          (:`<`
            (`/Engine/EditorBlueprintResources/StandardMacros.CompareFloat` (`self.Degrees`) 90.0
              (:`>`
                (`SceneComponent.K2_SetRelativeRotation` (`self.PaperFlipbook`) (struct :`Yaw` 180.0) false false :!label _label_3)
                (`PaperFlipbookComponent.SetFlipbook` (`self.PaperFlipbook`) (`|GetArrayItem` (select `/Game/RetroFpsAssets/Enemies/EnemyState` (`self.EnemyState`) :`NewEnumerator0` (`self.FlipbooksIdles`) :`NewEnumerator1` (`self.FlipbooksMoving`) :`NewEnumerator2` (`self.FlipbooksMeleeAttacks`) :`NewEnumerator3` (`self.FlipbooksRangedAttacks`)) 2)))
              (:`==`
                (goto _label_3))
              (:`<`
                (`/Engine/EditorBlueprintResources/StandardMacros.CompareFloat` (`self.Degrees`) 45.0
                  (:`>`
                    _)
                  (:`==`
                    _)
                  (:`<`
                    (goto _label)))
                (`SceneComponent.K2_SetRelativeRotation` (`self.PaperFlipbook`) (struct :`Yaw` 45.0) false false)
                (`PaperFlipbookComponent.SetFlipbook` (`self.PaperFlipbook`) (`|GetArrayItem` (select `/Game/RetroFpsAssets/Enemies/EnemyState` (`self.EnemyState`) :`NewEnumerator0` (`self.FlipbooksIdles`) :`NewEnumerator1` (`self.FlipbooksMoving`) :`NewEnumerator2` (`self.FlipbooksMeleeAttacks`) :`NewEnumerator3` (`self.FlipbooksRangedAttacks`)) 1))))))))
    (else
      (`/Engine/EditorBlueprintResources/StandardMacros.CompareFloat` (`self.Degrees`) 180.0
        (:`>`
          (`SceneComponent.K2_SetRelativeRotation` (`self.PaperFlipbook`) (struct :`Yaw` -45.0) false false :!label _label_4)
          (`PaperFlipbookComponent.SetFlipbook` (`self.PaperFlipbook`) (`|GetArrayItem` (select `/Game/RetroFpsAssets/Enemies/EnemyState` (`self.EnemyState`) :`NewEnumerator0` (`self.FlipbooksIdles`) :`NewEnumerator1` (`self.FlipbooksMoving`) :`NewEnumerator2` (`self.FlipbooksMeleeAttacks`) :`NewEnumerator3` (`self.FlipbooksRangedAttacks`)) 1)))
        (:`==`
          (goto _label_4))
        (:`<`
          (`/Engine/EditorBlueprintResources/StandardMacros.CompareFloat` (`self.Degrees`) 135.0
            (:`>`
              (`SceneComponent.K2_SetRelativeRotation` (`self.PaperFlipbook`) (struct :`Yaw` 90.0) false false :!label _label_5)
              (`PaperFlipbookComponent.SetFlipbook` (`self.PaperFlipbook`) (`|GetArrayItem` (select `/Game/RetroFpsAssets/Enemies/EnemyState` (`self.EnemyState`) :`NewEnumerator0` (`self.FlipbooksIdles`) :`NewEnumerator1` (`self.FlipbooksMoving`) :`NewEnumerator2` (`self.FlipbooksMeleeAttacks`) :`NewEnumerator3` (`self.FlipbooksRangedAttacks`)) 4)))
            (:`==`
              (goto _label_5))
            (:`<`
              (`/Engine/EditorBlueprintResources/StandardMacros.CompareFloat` (`self.Degrees`) 90.0
                (:`>`
                  (`SceneComponent.K2_SetRelativeRotation` (`self.PaperFlipbook`) (struct :`Yaw` 45.0) false false :!label _label_6)
                  (`PaperFlipbookComponent.SetFlipbook` (`self.PaperFlipbook`) (`|GetArrayItem` (select `/Game/RetroFpsAssets/Enemies/EnemyState` (`self.EnemyState`) :`NewEnumerator0` (`self.FlipbooksIdles`) :`NewEnumerator1` (`self.FlipbooksMoving`) :`NewEnumerator2` (`self.FlipbooksMeleeAttacks`) :`NewEnumerator3` (`self.FlipbooksRangedAttacks`)) 5)))
                (:`==`
                  (goto _label_6))
                (:`<`
                  (`/Engine/EditorBlueprintResources/StandardMacros.CompareFloat` (`self.Degrees`) 45.0
                    (:`>`
                      _)
                    (:`==`
                      _)
                    (:`<`
                      (goto _label_4)))
                  (`SceneComponent.K2_SetRelativeRotation` :`self` (`self.PaperFlipbook`))
                  (`PaperFlipbookComponent.SetFlipbook` (`self.PaperFlipbook`) (`|GetArrayItem` (select `/Game/RetroFpsAssets/Enemies/EnemyState` (`self.EnemyState`) :`NewEnumerator0` (`self.FlipbooksIdles`) :`NewEnumerator1` (`self.FlipbooksMoving`) :`NewEnumerator2` (`self.FlipbooksMeleeAttacks`) :`NewEnumerator3` (`self.FlipbooksRangedAttacks`)) 6)))))))))))

(event `RotateTowardsPlayer`
  (`self.K2_SetActorRotation` (`KismetMathLibrary.RInterpTo` (`self.K2_GetActorRotation`) (`KismetMathLibrary.FindLookAtRotation` (`self.K2_GetActorLocation`) (`self.K2_GetActorLocation` (`GameplayStatics.GetPlayerCharacter` 0))) (`GameplayStatics.GetWorldDeltaSeconds`) (`self.RotationSpeed`))))

(event `self.PawnSensing.OnSeePawn`
  (params (Pawn :type "Pawn Object Reference"))
  (cast `/Game/FirstPerson/Blueprints/BP_FirstPersonCharacter` Pawn)
  (set `self.CanSeePlayer` true)
  (`BlackboardComponent.SetValueAsBool` (`AIBlueprintHelperLibrary.GetBlackboard` null) "CanSeePlayer" true)
  (`KismetSystemLibrary.RetriggerableDelay` 0.7)
  (set `self.CanSeePlayer` false)
  (`BlackboardComponent.SetValueAsBool` (`AIBlueprintHelperLibrary.GetBlackboard` null) "CanSeePlayer" false))

(event `SpawnProjectile`
  (set `self.IsAttacking` true)
  (set `self.AttackState` "NewEnumerator1")
  (`MovementComponent.StopMovementImmediately` (`self.CharacterMovement`))
  (`KismetSystemLibrary.RetriggerableDelay` 0.5)
  (`|SpawnActorFromClass` "/Game/RetroFpsAssets/Enemies/EnemyProjectile_BP.EnemyProjectile_BP_C" (`SceneComponent.K2_GetComponentToWorld` (`self.ProjectileSpawn`)) "Undefined" "MultiplyWithRoot" null null)
  (set `self.IsAttacking` false))

(event `MeleerAttack`
  (bind _returnvalue (`self.K2_GetActorLocation`))
  (set `self.IsAttacking` true)
  (set `self.AttackState` "NewEnumerator0")
  (`KismetSystemLibrary.RetriggerableDelay` 0.5)
  (bind _outhit (`KismetSystemLibrary.LineTraceSingleForObjects` _returnvalue (+ _returnvalue (* (`self.GetActorForwardVector`) 150.0)) (`|MakeArray` "ObjectTypeQuery3" :!type "EObjectTypeQuery Enum") false (`|MakeArray` self :!type "Actor Object Reference") "ForDuration"))
  (bind (_bblockinghit _binitialoverlap _time _distance _location _impactpoint _normal _impactnormal _physmat _hitactor) (`GameplayStatics.BreakHitResult` _outhit))
  (if (== _hitactor (`GameplayStatics.GetPlayerCharacter` 0))
    (`GameplayStatics.ApplyDamage` _hitactor (`self.EnemyDamage`)))
  (set `self.IsAttacking` false))

(event `self.ReceiveAnyDamage`
  (params (Damage :type "Float (single-precision)") (DamageType :type "DamageType Object Reference") (InstigatedBy :type "Controller Object Reference") (DamageCauser :type "Actor Object Reference"))
  (bind _output_get (set `self.Health` (- (`self.Health`) Damage)))
  (if (<= _output_get 0.0)
    (`self.K2_DestroyActor`)
    (`/Engine/EditorBlueprintResources/StandardMacros.IncrementInt` (`/Game/RetroFpsAssets/Blueprints/Stats_BPC.KillCount` (`/Game/FirstPerson/Blueprints/BP_FirstPersonCharacter.Stats_BPC` (`self.PlayerReference`))))))

(fn `UserConstructionScript`)