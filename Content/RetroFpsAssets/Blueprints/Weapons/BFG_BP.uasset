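; BFG weapon Blueprint for a retro FPS, animated with flipbooks and fired at a cost of 30 Cell ammo per shot.
; ShootWeapon checks the player's ammo, then plays the fire flipbook and waits for its length before launching the projectile, deducting ammo and updating the HUD.
; A DoOnce gate blocks repeat shots until the weapon returns to its idle flipbook and ResetFire reopens it.
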(event `self.ShootWeapon`
  (bind _weaponflipbook (`self.WeaponFlipbook`))
  (bind _playerreference (`self.PlayerReference`))
  (bind _ammo_bpc (`/Game/FirstPerson/Blueprints/BP_FirstPersonCharacter.Ammo_BPC` _playerreference))
  (if (>= (`/Game/RetroFpsAssets/Blueprints/Ammo_BPC.Cell` (`/Game/FirstPerson/Blueprints/BP_FirstPersonCharacter.Ammo_BPC` (`self.PlayerReference`))) 30)
    (`/Engine/EditorBlueprintResources/StandardMacros.DoOnce` false :!label _label
      (:`Completed`
        (`PaperFlipbookComponent.SetFlipbook` _weaponflipbook "/Game/RetroFpsAssets/Sprites/Weapons/BFG/BFGFire.BFGFire")
        (`KismetSystemLibrary.Delay` (`PaperFlipbookComponent.GetFlipbookLength` _weaponflipbook))
        (`self.FireProjectile` 4000.0)
        (set `/Game/RetroFpsAssets/Blueprints/Ammo_BPC.Cell` (- (`/Game/RetroFpsAssets/Blueprints/Ammo_BPC.Cell` _ammo_bpc) 30) _ammo_bpc)
        (`/Game/RetroFpsAssets/Blueprints/UI/PlayerHUD_WB.UpdateCellAmmo` (`/Game/FirstPerson/Blueprints/BP_FirstPersonCharacter.PlayerHUDReference` _playerreference))
        (`PaperFlipbookComponent.SetFlipbook` (`self.WeaponFlipbook`) "/Game/RetroFpsAssets/Sprites/Weapons/BFG/BFGIdle.BFGIdle")
        (`self.ResetFire`)))))

(event `ResetFire`
  (goto _label :!via `Reset`))

(fn `UserConstructionScript`
  (`parent.UserConstructionScript`))