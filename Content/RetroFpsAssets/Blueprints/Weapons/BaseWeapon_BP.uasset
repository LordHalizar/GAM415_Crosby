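; Base weapon Blueprint for a retro FPS, providing shared firing and ammo logic with empty ShootWeapon and StopShooting events.
; BeginPlay caches the first-person player, whose ammo component backs HasEnoughAmmo? and DecreaseAmmo, switched on AmmoType (bullet, shell, rocket, cell), with decrements refreshing the HUD.
; FireWeapon applies hitscan damage through a debug-drawn line trace.
; FireProjectile spawns a projectile given the weapon's damage and a supplied speed.
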(event `ShootWeapon`)

(event `StopShooting`)

(event `self.ReceiveBeginPlay`
  (bind _asbp_first_person_character (cast `/Game/FirstPerson/Blueprints/BP_FirstPersonCharacter` (`GameplayStatics.GetPlayerCharacter` 0)))
  (set `self.PlayerReference` _asbp_first_person_character))

(event `DecreaseAmmo`
  (switch `/Game/RetroFpsAssets/Blueprints/Weapons/Ammo` (`self.AmmoType`)
    (:`NewEnumerator0`
      (`/Engine/EditorBlueprintResources/StandardMacros.DecrementInt` (`/Game/RetroFpsAssets/Blueprints/Ammo_BPC.Bullet` (`/Game/FirstPerson/Blueprints/BP_FirstPersonCharacter.Ammo_BPC` (`self.PlayerReference`)))
        (:`  `
          (`/Game/RetroFpsAssets/Blueprints/UI/PlayerHUD_WB.UpdateBulletAmmo` (`/Game/FirstPerson/Blueprints/BP_FirstPersonCharacter.PlayerHUDReference` (`self.PlayerReference`))))))
    (:`NewEnumerator1`
      (`/Engine/EditorBlueprintResources/StandardMacros.DecrementInt` (`/Game/RetroFpsAssets/Blueprints/Ammo_BPC.Shell` (`/Game/FirstPerson/Blueprints/BP_FirstPersonCharacter.Ammo_BPC` (`self.PlayerReference`)))
        (:`  `
          (`/Game/RetroFpsAssets/Blueprints/UI/PlayerHUD_WB.UpdateShellAmo` (`/Game/FirstPerson/Blueprints/BP_FirstPersonCharacter.PlayerHUDReference` (`self.PlayerReference`))))))
    (:`NewEnumerator2`
      (`/Engine/EditorBlueprintResources/StandardMacros.DecrementInt` (`/Game/RetroFpsAssets/Blueprints/Ammo_BPC.Rocket` (`/Game/FirstPerson/Blueprints/BP_FirstPersonCharacter.Ammo_BPC` (`self.PlayerReference`)))
        (:`  `
          (`/Game/RetroFpsAssets/Blueprints/UI/PlayerHUD_WB.UpdateRocketAmmo` (`/Game/FirstPerson/Blueprints/BP_FirstPersonCharacter.PlayerHUDReference` (`self.PlayerReference`))))))
    (:`NewEnumerator3`
      (`/Engine/EditorBlueprintResources/StandardMacros.DecrementInt` (`/Game/RetroFpsAssets/Blueprints/Ammo_BPC.Cell` (`/Game/FirstPerson/Blueprints/BP_FirstPersonCharacter.Ammo_BPC` (`self.PlayerReference`)))
        (:`  `
          (`/Game/RetroFpsAssets/Blueprints/UI/PlayerHUD_WB.UpdateCellAmmo` (`/Game/FirstPerson/Blueprints/BP_FirstPersonCharacter.PlayerHUDReference` (`self.PlayerReference`))))))))

(fn `FireProjectile`
  (params (ProjectileSpeed :type "Float (double-precision)"))
  (`|SpawnActorFromClass` (`self.Projectile`) (`SceneComponent.K2_GetComponentToWorld` (`self.ProjectileTransform`)) "Undefined" "MultiplyWithRoot" null (`self.WeaponDamage`) ProjectileSpeed null))

(fn `FireWeapon`
  (bind _linetrace (`self.LineTrace`))
  (bind _returnvalue (`SceneComponent.K2_GetComponentLocation` _linetrace))
  (bind (_outhit _returnvalue_2) (`KismetSystemLibrary.LineTraceSingleForObjects` _returnvalue (+ _returnvalue (* (`KismetMathLibrary.GetForwardVector` (`SceneComponent.K2_GetComponentRotation` _linetrace)) (`self.LineTraceDistance`))) (`|MakeArray` "ObjectTypeQuery1" "ObjectTypeQuery2" "ObjectTypeQuery3" :!type "EObjectTypeQuery Enum") false (`|MakeArray` self (`GameplayStatics.GetPlayerCharacter` 0) :!type "Actor Object Reference") "ForDuration"))
  (if _returnvalue_2
    (`GameplayStatics.ApplyDamage` (`.HitActor` (`GameplayStatics.BreakHitResult` _outhit)) (`self.WeaponDamage`))))

(fn `HasEnoughAmmo?`
  (returns (HasAmmo :type Boolean))
  (switch `/Game/RetroFpsAssets/Blueprints/Weapons/Ammo` (`self.AmmoType`)
    (:`NewEnumerator0`
      (if (> (`/Game/RetroFpsAssets/Blueprints/Ammo_BPC.Bullet` (`/Game/FirstPerson/Blueprints/BP_FirstPersonCharacter.Ammo_BPC` (`self.PlayerReference`))) 0)
        (return true)
        (else
          (return false))))
    (:`NewEnumerator1`
      (if (> (`/Game/RetroFpsAssets/Blueprints/Ammo_BPC.Shell` (`/Game/FirstPerson/Blueprints/BP_FirstPersonCharacter.Ammo_BPC` (`self.PlayerReference`))) 0)
        (return true)
        (else
          (return false))))
    (:`NewEnumerator2`
      (if (> (`/Game/RetroFpsAssets/Blueprints/Ammo_BPC.Rocket` (`/Game/FirstPerson/Blueprints/BP_FirstPersonCharacter.Ammo_BPC` (`self.PlayerReference`))) 0)
        (return true)
        (else
          (return false))))
    (:`NewEnumerator3`
      (if (> (`/Game/RetroFpsAssets/Blueprints/Ammo_BPC.Cell` (`/Game/FirstPerson/Blueprints/BP_FirstPersonCharacter.Ammo_BPC` (`self.PlayerReference`))) 0)
        (return true)
        (else
          (return false))))))

(fn `UserConstructionScript`)