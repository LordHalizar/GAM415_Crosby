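; Retro FPS weapon pickup that shows a billboard sprite and hands the player a weapon.
; The Construction Script maps the Weapon selection to its Paper2D sprite and weapon class.
; Tick yaws the actor toward the player, keeping the flat sprite facing them.
; On sphere overlap with BP_FirstPersonCharacter, it passes the class to PickupWeapon and destroys itself.
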(event `self.ReceiveTick`
  (params (DeltaSeconds :type "Float (single-precision)"))
  (bind (_returnvalue_roll _returnvalue_pitch _returnvalue_yaw) (`KismetMathLibrary.BreakRotator` (`KismetMathLibrary.FindLookAtRotation` (`self.K2_GetActorLocation`) (`self.K2_GetActorLocation` (`GameplayStatics.GetPlayerCharacter` 0)))))
  (`self.K2_SetActorRotation` (`KismetMathLibrary.MakeRotator` 0.0 0.0 _returnvalue_yaw)))

(event `self.SphereCollision.OnComponentBeginOverlap`
  (params (OverlappedComponent :type "PrimitiveComponent Object Reference") (OtherActor :type "Actor Object Reference") (OtherComp :type "PrimitiveComponent Object Reference") (OtherBodyIndex :type Integer) (bFromSweep :type Boolean) (SweepResult :type "HitResult Structure (by ref)"))
  (bind _asbp_first_person_character (cast `/Game/FirstPerson/Blueprints/BP_FirstPersonCharacter` OtherActor))
  (`/Game/FirstPerson/Blueprints/BP_FirstPersonCharacter.PickupWeapon` _asbp_first_person_character (`self.WeaponClass`))
  (`self.K2_DestroyActor`))

(fn `UserConstructionScript`
  (switch `/Game/RetroFpsAssets/Blueprints/Weapons/Weapon` (`self.Weapon`)
    (:`NewEnumerator0`
      (`PaperSpriteComponent.SetSprite` (`self.PaperSprite`) "/Game/RetroFpsAssets/Sprites/Weapons/Shotgun/ShotgunSprite.ShotgunSprite")
      (set `self.WeaponClass` "/Game/RetroFpsAssets/Blueprints/Weapons/Shotgun_BP.Shotgun_BP_C"))
    (:`NewEnumerator1`
      (`PaperSpriteComponent.SetSprite` (`self.PaperSprite`) "/Game/RetroFpsAssets/Sprites/Weapons/MiniGun/MinigunSprite.MinigunSprite")
      (set `self.WeaponClass` "/Game/RetroFpsAssets/Blueprints/Weapons/Minigun_BP.Minigun_BP_C"))
    (:`NewEnumerator2`
      (`PaperSpriteComponent.SetSprite` (`self.PaperSprite`) "/Game/RetroFpsAssets/Sprites/Weapons/PlasmaGun/PlasmaRifleSprite.PlasmaRifleSprite")
      (set `self.WeaponClass` "/Game/RetroFpsAssets/Blueprints/Weapons/Plasmagun_BP.Plasmagun_BP_C"))
    (:`NewEnumerator3`
      (`PaperSpriteComponent.SetSprite` (`self.PaperSprite`) "/Game/RetroFpsAssets/Sprites/Weapons/RPG/RPGSprite.RPGSprite")
      (set `self.WeaponClass` "/Game/RetroFpsAssets/Blueprints/Weapons/RPG_BP.RPG_BP_C"))
    (:`NewEnumerator4`
      (`PaperSpriteComponent.SetSprite` (`self.PaperSprite`) "/Game/RetroFpsAssets/Sprites/Weapons/BFG/BFGSprite.BFGSprite")
      (set `self.WeaponClass` "/Game/RetroFpsAssets/Blueprints/Weapons/BFG_BP.BFG_BP_C"))
    (:`NewEnumerator5`
      (`PaperSpriteComponent.SetSprite` (`self.PaperSprite`) "/Game/RetroFpsAssets/Sprites/Weapons/Chainsaw/ChainsawSprite.ChainsawSprite")
      (set `self.WeaponClass` "/Game/RetroFpsAssets/Blueprints/Weapons/Chainsaw_BP.Chainsaw_BP_C"))))