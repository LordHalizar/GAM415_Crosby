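; Level portal actor that moves the first-person character to the next ProjectA map when they overlap its LevelPortal component.
; On BeginPlay it stores and prints the current level name.
; On overlap, a hardcoded if/else chain compares that name and opens the next map in the order Starter, Portal, Decal, Terrain.
; Terrain is the end of the chain and opens nothing.
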(event `self.ReceiveBeginPlay`
  (bind _returnvalue (`GameplayStatics.GetCurrentLevelName` true))
  (bind _output_get (set `self.Level Name` (`KismetStringLibrary.Conv_StringToName` _returnvalue)))
  (`KismetSystemLibrary.PrintString` (`KismetStringLibrary.Conv_NameToString` _output_get)))

(event `self.LevelPortal.OnComponentBeginOverlap`
  (params (OverlappedComponent :type "PrimitiveComponent Object Reference") (OtherActor :type "Actor Object Reference") (OtherComp :type "PrimitiveComponent Object Reference") (OtherBodyIndex :type Integer) (bFromSweep :type Boolean) (SweepResult :type "HitResult Structure (by ref)"))
  (bind _returnvalue (`KismetTextLibrary.Conv_StringToText` "ProjectAMap_Portal"))
  (bind _returnvalue_2 (`KismetTextLibrary.Conv_StringToText` "ProjectAMap_Decal"))
  (bind _returnvalue_3 (`KismetTextLibrary.Conv_StringToText` "ProjectAMap_Terrain"))
  (bind _returnvalue_4 (`KismetTextLibrary.Conv_NameToText` (`self.Level Name`)))
  (cast `FirstPerson415Character` OtherActor)
  (`|ExecutionSequence`
    (:`then_0`
      (if (`KismetTextLibrary.EqualEqual_TextText` _returnvalue_4 (`KismetTextLibrary.Conv_StringToText` "ProjectAMap_Starter"))
        (bind _output_get (set `self.Level Name` (`KismetStringLibrary.Conv_StringToName` (`KismetTextLibrary.Conv_TextToString` _returnvalue))))
        (`GameplayStatics.OpenLevel` _output_get)
        (elif (`KismetTextLibrary.EqualEqual_TextText` _returnvalue_4 _returnvalue)
          (bind _output_get_2 (set `self.Level Name` (`KismetStringLibrary.Conv_StringToName` (`KismetTextLibrary.Conv_TextToString` _returnvalue_2))))
          (`GameplayStatics.OpenLevel` _output_get_2)
          (elif (`KismetTextLibrary.EqualEqual_TextText` _returnvalue_4 _returnvalue_2)
            (bind _output_get_3 (set `self.Level Name` (`KismetStringLibrary.Conv_StringToName` (`KismetTextLibrary.Conv_TextToString` _returnvalue_3))))
            (`GameplayStatics.OpenLevel` _output_get_3)
            (elif (`KismetTextLibrary.EqualEqual_TextText` _returnvalue_4 _returnvalue_3)
              _)))))))

(fn `UserConstructionScript`)