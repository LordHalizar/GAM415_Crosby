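; EnemyRoom_BP is a room Blueprint in the dungeon generation system that places an enemy when play begins.
; BeginPlay runs the parent logic, then spawns one BaseEnemy_BP at the Floor component's world location, nudged one unit along the floor's up vector.
; The construction script only defers to its parent, and the Tick and overlap events are unused stubs.
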(event `self.ReceiveBeginPlay`
  (bind _floor (`self.Floor`))
  (`parent.ReceiveBeginPlay`)
  (`|SpawnActorFromClass` "/Game/RetroFpsAssets/Enemies/BaseEnemy_BP.BaseEnemy_BP_C" (`KismetMathLibrary.MakeTransform` (+ (+ (`SceneComponent.K2_GetComponentLocation` _floor) (0.0 0.0 0.0)) (* (`KismetMathLibrary.GetUpVector` (`SceneComponent.K2_GetComponentRotation` _floor)) 1.0))) "Undefined" "MultiplyWithRoot" null null))

(fn `UserConstructionScript`
  (`parent.UserConstructionScript`))