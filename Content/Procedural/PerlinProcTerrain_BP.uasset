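; Perlin procedural terrain actor that randomizes its noise scale when the first-person player character overlaps it.
; The overlap calls a custom event that sets NoiseScale to a random float, then prints the value.
; Tick only reassigns NoiseScale to itself, and no mesh generation happens in this graph.
; Disconnected nodes would size a box extent from the X and Y grid sizes but never run.
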(event Custom|SetNoiseScale
  (Variables|Default|SetNoiseScale (Math|Random|RandomFloat)))

(event EventBeginPlay)

(event Collision|EventActorBeginOverlap
  (params (OtherActor :type Actor%20Object%20Reference))
  (Utilities|Casting|CastToFirstPerson415Character OtherActor)
  (CallFunction|SetNoiseScale)
  (Development|PrintString (Utilities|String|ToString(Float) (Variables|Default|GetNoiseScale))))

(event EventTick
  (params (DeltaSeconds :type Float%20%28single-precision%29))
  (Variables|Default|SetNoiseScale (Variables|Default|GetNoiseScale)))

(event Input|KeyboardEvents|DebugKeyE
  (params (Key :type Key%20Structure :default "None") (ActionValue :type Input%20Action%20Value%20Structure)))

(fn ConstructionScript)