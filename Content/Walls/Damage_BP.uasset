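; Damage field actor for walls that moves its Field System component when a switch activates it, likely to break Chaos destructibles.
; SwitchActivated plays the MoveDamage timeline, lerping the component from LocStart to LocEnd.
; ResetDamage waits briefly, then reverses the timeline to move it back.
; LocStart is captured in world space at BeginPlay, but the lerp result is applied as a relative location.
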(event `self.ReceiveActorBeginOverlap`
  (params (OtherActor :type "Actor Object Reference")))

(event `self.ReceiveBeginPlay`
  (`parent.ReceiveBeginPlay`)
  (set `self.Loc_Start` (`SceneComponent.K2_GetComponentLocation` (`self.FieldSystemComponent`))))

(event `SwitchActivated`
  (bind (_direction _movement) (`Timeline|Move Damage` :!label _label)
    (:`Update`
      (`SceneComponent.K2_SetRelativeLocation` (`self.FieldSystemComponent`) (`KismetMathLibrary.VLerp` (`self.Loc_Start`) (`self.Loc_End`) _movement) false false))))

(event `ResetDamage`
  (`KismetSystemLibrary.Delay` 2.5)
  (goto _label :!via `Reverse`))

(fn `UserConstructionScript`
  (`parent.UserConstructionScript`))