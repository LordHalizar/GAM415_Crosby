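; Field system actor for walls that, judging by its name, supplies a moving damage force when a switch is activated.
; BeginPlay caches the component's world position and treats LocEnd as an offset, converting it into an absolute end point.
; SwitchActivated plays the MoveDamage timeline, lerping the FieldSystemComponent between both points through SetRelativeLocation, despite their world-space origin.
; ResetDamage is an empty stub.
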(event `self.ReceiveActorBeginOverlap`
  (params (OtherActor :type "Actor Object Reference")))

(event `self.ReceiveBeginPlay`
  (`parent.ReceiveBeginPlay`)
  (set `self.Loc_Start` (`SceneComponent.K2_GetComponentLocation` (`self.FieldSystemComponent`)))
  (set `self.Loc_End` (`KismetMathLibrary.MakeVector` (+ (.x (`self.Loc_Start`)) (.x (`self.Loc_End`))) (+ (.y (`self.Loc_Start`)) (.y (`self.Loc_End`))) (+ (.z (`self.Loc_Start`)) (.z (`self.Loc_End`))))))

(event `SwitchActivated`
  (bind (_direction _movement) (`Timeline|Move Damage`)
    (:`Update`
      (`SceneComponent.K2_SetRelativeLocation` (`self.FieldSystemComponent`) (`KismetMathLibrary.VLerp` (`self.Loc_Start`) (`self.Loc_End`) _movement) false false))))

(event `ResetDamage`)

(fn `UserConstructionScript`
  (`parent.UserConstructionScript`))